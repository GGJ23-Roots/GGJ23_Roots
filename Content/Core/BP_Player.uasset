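; Player character with a grappling cable that latches onto interactive props and drags them along.
; LaunchCable targets props within an aim cone, scored by dot product times distance, then a timeline extends a runtime-created cable, sphere-checking for a hit.
; Tick pulls the grabbed mesh with distance-scaled impulses, releasing it beyond maximum range.
; Also handles timed recovery from physics knockdown, proximity prop pop-up text and caching the loaded level.
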(event OnComponentBeginOverlap(Sphere)
  (params (OverlappedComponent :type Primitive%20Component%20Object%20Reference) (OtherActor :type Actor%20Object%20Reference) (OtherComp :type Primitive%20Component%20Object%20Reference) (OtherBodyIndex :type Integer) (bFromSweep :type Boolean) (SweepResult :type Hit%20Result%20Structure%20%28by%20ref%29))
  (bind _asbp_interactive_props (Utilities|Casting|CastToBP_InteractiveProps OtherActor))
  (Default|PopUpText _asbp_interactive_props "Forward"))

(event OnComponentEndOverlap(Sphere)
  (params (OverlappedComponent :type Primitive%20Component%20Object%20Reference) (OtherActor :type Actor%20Object%20Reference) (OtherComp :type Primitive%20Component%20Object%20Reference) (OtherBodyIndex :type Integer))
  (bind _asbp_interactive_props (Utilities|Casting|CastToBP_InteractiveProps OtherActor))
  (Default|PopUpText _asbp_interactive_props "Reverse"))

(event Custom|GetBackUp
  (bind _capsulecomponent (Variables|Collision|GetCapsuleComponent))
  (if (not (Variables|Default|GetHit))
    (Variables|Default|SetHit true)
    (Utilities|FlowControl|Delay 2.0)
    (Class|PrimitiveComponent|SetAllPhysicsLinearVelocity _capsulecomponent "0, 0, 0" false)
    (Class|PrimitiveComponent|SetAllPhysicsAngularVelocityinDegrees _capsulecomponent (Math|Vector|MakeVector 0.0 0.0 0.0) false)
    (Physics|AddImpulse (Variables|Collision|GetCapsuleComponent) "0.000000,0.000000,500.000000" "None" true)
    (bind _rotation (Timeline|Timeline PlayFromStart)
      (:Update
        (Transformation|SetWorldRotation (Variables|Collision|GetCapsuleComponent) (Math|Rotator|Lerp(Rotator) (Transformation|GetWorldRotation (Variables|Collision|GetCapsuleComponent)) "0, 0, 0" _rotation true) false false))
      (:Finished
        (Physics|SetSimulatePhysics (Variables|Collision|GetCapsuleComponent) false)
        (Variables|Default|SetHit false)))))

(event Custom|LaunchCable
  ;[1 1 1] GrabClosestComponent (dotProduct*dist) or miss
  (if (Variables|GrabbingSetup|GetCanLaunchGrab)
    (Variables|GrabbingSetup|SetCanLaunchGrab false)
    (CallFunction|SetupGrabComponents)
    (bind _bestgrab (CallFunction|CalculateCloserGrab))
    (Variables|GrabbingSetup|SetBestGrab _bestgrab)
    (bind _bestgrab_2 (Variables|GrabbingSetup|GetBestGrab)
      (:then
        (Variables|GrabbingSetup|SetLocationToGrab (Transformation|GetActorLocation _bestgrab_2))
        (bind _locationratio (Timeline|LaunchingTime PlayFromStart)
          (:Update
            (Transformation|SetWorldLocation (Variables|Default|GetEndCable) (Math|Vector|Lerp(Vector) (Transformation|GetActorLocation) (Variables|GrabbingSetup|GetLocationToGrab) _locationratio) false false)
            (bind (_outactors _returnvalue) (Collision|SphereOverlapActors (Math|Vector|Lerp(Vector) (Transformation|GetActorLocation) (Variables|GrabbingSetup|GetLocationToGrab) _locationratio) 1e+01 (Utilities|Array|MakeArray "ObjectTypeQuery1" "ObjectTypeQuery2" "ObjectTypeQuery4") (Variables|Default|GetClassToGrab)))
            (if _returnvalue
              (bind _asbp_interactive_props (Utilities|Casting|CastToBP_InteractiveProps (Utilities|Array|Get(acopy) _outactors)))
              (bind _output_get (Variables|Default|SetGrabbedComponent (Variables|/Game/Blueprints/Props/BP_Props.BP_Props_C|GetStaticMesh _asbp_interactive_props)))
              (Class|CableComponent|SetAttachEndtoComponent (Variables|Default|GetCableRef) _output_get "None")
              (Components|DestroyComponent (Variables|Default|GetEndCable))
              (Variables|GrabbingSetup|SetCanLaunchGrab true)
              (Audio|Components|Audio|Stop (Variables|Default|GetLaunchingTime))))
          (:Finished
            (Variables|GrabbingSetup|SetCanLaunchGrab true)
            (Components|DestroyComponent (Variables|Default|GetCableRef))
            (Components|DestroyComponent (Variables|Default|GetEndCable)))))
      (:else
        (Variables|GrabbingSetup|SetLocationToGrab (+ (* (Transformation|GetActorForwardVector) (Variables|GrabbingSetup|GetDistanceCable)) (Transformation|GetActorLocation)))
        (Timeline|LaunchingTime PlayFromStart)))))

(event EventTick
  (params (DeltaSeconds :type Float%20%28single-precision%29))
  (CallFunction|ManageGrabbedPhysics))

(event EventBeginPlay
  ;[1 1 1] GrapplingTimelineSpeed
  (Components|Timeline|SetPlayRate (Variables|Default|GetLaunchingTime) (/ 1.0 (Variables|GrabbingSetup|GetGrapplingSpeed)))
  (bind _outactors (Actor|GetAllActorsOfClass "/Game/Blueprints/BP_Level.BP_Level_C"))
  (bind _array_element (Utilities|Array|ForEachLoopwithBreak _outactors)
    (:LoopBody
      (if (Variables|/Game/Blueprints/BP_Level.BP_Level_C|GetLoaded _array_element)
        (Variables|Default|SetCurrentLevel _array_element)))))

(fn ConstructionScript)

(fn ManageGrabbedPhysics
  (bind _grabbedcomponent (Variables|Default|GetGrabbedComponent)
    (:then
      (Utilities|FlowControl|Sequence
        (:then_0
          (LocalVariables|SetGrabbedLocation (Transformation|GetWorldLocation _grabbedcomponent))
          (LocalVariables|SetPlayerLocation (Transformation|GetActorLocation))
          (if (>= (Math|Vector|Distance2D(Vector) (LocalVariables|GetGrabbedLocation) (LocalVariables|GetPlayerLocation)) (Variables|GrabbedObject|GetMinDistanceGrabbed))
            (Physics|AddImpulse (Variables|Default|GetGrabbedComponent) (* (Math|Vector|GetUnitDirection(Vector) (LocalVariables|GetGrabbedLocation) (LocalVariables|GetPlayerLocation)) (Variables|GrabbedObject|GetImpulseGrabbed) (* (/ (Math|Vector|Distance2D(Vector) (LocalVariables|GetGrabbedLocation) (LocalVariables|GetPlayerLocation)) (Variables|Default|GetMaxDistanceGrabbed)) (Variables|Default|GetRatioDistanceGrabbed))) "None" true)))
        (:then_1
          (if (>= (Math|Vector|Distance2D(Vector) (LocalVariables|GetGrabbedLocation) (LocalVariables|GetPlayerLocation)) (Variables|Default|GetMaxDistanceGrabbed))
            (CallFunction|ReleaseComponent)))))
    (:else)))

(fn ReleaseComponent
  (Variables|Default|GetGrabbedComponent
    (:then
      (Variables|Default|SetGrabbedComponent 0)
      (Components|DestroyComponent (Variables|Default|GetCableRef)))
    (:else)))

(fn CalculateCloserGrab
  (bind _truedirection (Variables|Default|GetTrueDirection))
  ;[1 1 1] Pour tous les interactibles a distance de grab du player
  (bind _outactors (Collision|SphereOverlapActors (Transformation|GetActorLocation) (Variables|GrabbingSetup|GetDistanceCable) (Utilities|Array|MakeArray "ObjectTypeQuery1" "ObjectTypeQuery2" "ObjectTypeQuery4") (Variables|Default|GetClassToGrab)))
  (for _array_element _outactors
    (if (and (> (Math|Vector|DotProduct (select (Math|Vector|VectorIsNearlyZero _truedirection) (Transformation|GetActorForwardVector) _truedirection) (Math|Vector|GetUnitDirection(Vector) (Transformation|GetActorLocation) (Transformation|GetActorLocation _array_element))) (Variables|GrabbingSetup|GetMaxAngleGrab)) (> (* (Transformation|GetHorizontalDistanceTo _array_element self) (Math|Vector|DotProduct (select (Math|Vector|VectorIsNearlyZero _truedirection) (Transformation|GetActorForwardVector) _truedirection) (Math|Vector|GetUnitDirection(Vector) (Transformation|GetActorLocation) (Transformation|GetActorLocation _array_element)))) (LocalVariables|GetBestActorValue)))
      (LocalVariables|SetBestActor _array_element)
      (LocalVariables|SetBestActorValue (* (Transformation|GetHorizontalDistanceTo _array_element self) (Math|Vector|DotProduct (select (Math|Vector|VectorIsNearlyZero _truedirection) (Transformation|GetActorForwardVector) _truedirection) (Math|Vector|GetUnitDirection(Vector) (Transformation|GetActorLocation) (Transformation|GetActorLocation _array_element)))))))
  (return (LocalVariables|GetBestActor)))

(fn SetupGrabComponents
  (bind _returnvalue (AddComponent|AddSceneComponent false))
  (Variables|Default|SetEndCable _returnvalue)
  (bind _returnvalue_2 (AddComponent|AddCableComponent false))
  (bind _output_get (Variables|Default|SetCableRef _returnvalue_2))
  (Transformation|AttachComponentToComponent _output_get (Variables|Character|GetMesh) "None" "KeepRelative" "KeepRelative" "KeepRelative" true)
  (Class|CableComponent|SetAttachEndtoComponent _output_get (Variables|Default|GetEndCable) "None"))