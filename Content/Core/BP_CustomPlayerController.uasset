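; Player controller that turns Enhanced Input into BP_Player actions and creates the master UI widget.
; BeginPlay adds gamepad and culture-based keyboard mappings (AZERTY for French, otherwise QWERTY) and caches the pawn.
; Movement follows world axes rotated 45 degrees; dash launches along capsule forward with a cooldown.
; Grab toggles cable launch and release, while OpenFolder triggers the best nearby interactive prop and logs it to the UI history.
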(event Input|EnhancedActionEvents|EnhancedInputActionIA_Move
  (params (ActionValue :type Vector%202D%20Structure) (ElapsedSeconds :type Float%20%28double-precision%29) (TriggeredSeconds :type Float%20%28double-precision%29) (InputAction :type Input%20Action%20Object%20Reference :default "/Game/Core/Inputs/IA_Move.IA_Move"))
  ;[1 1 1] Movement player in world direction
  (:Triggered
    (Pawn|Input|AddMovementInput (Variables|Default|GetPlayerRef) (Math|Vector|RotateVector "1.000000,0.000000,0.000000" "0.000000,-45.000000,0.000000") (.x ActionValue) false)
    (Pawn|Input|AddMovementInput (Variables|Default|GetPlayerRef) (Math|Vector|RotateVector "0.000000,1.000000,0.000000" "0.000000,-45.000000,0.000000") (.y ActionValue) false)
    (Variables|/Game/Core/BP_Player.BP_Player_C|SetTrueDirection (Variables|Default|GetPlayerRef) (Math|Vector|MakeVector (.x ActionValue) (.y ActionValue) 0.0)))
  (:Completed
    (Variables|/Game/Core/BP_Player.BP_Player_C|SetTrueDirection (Variables|Default|GetPlayerRef) "0, 0, 0")))

(event Input|EnhancedActionEvents|EnhancedInputActionIA_Dash
  (params (ActionValue :type Boolean) (ElapsedSeconds :type Float%20%28double-precision%29) (TriggeredSeconds :type Float%20%28double-precision%29) (InputAction :type Input%20Action%20Object%20Reference :default "/Game/Core/Inputs/IA_Dash.IA_Dash"))
  ;[1 1 1] Special interaction
  (:Started
    (if (Variables|Default|GetCanDash)
      (Variables|Default|SetCanDash false)
      (Character|LaunchCharacter (Variables|Default|GetPlayerRef) (* (Math|Vector|GetForwardVector (Variables|/Script/Engine.Character|GetCapsuleComponent (Variables|Default|GetPlayerRef))) (Variables|Default|GetDashForce)) true false)
      (Utilities|FlowControl|Delay (Variables|Default|GetDashCoolDown))
      (Variables|Default|SetCanDash true))))

(event Input|EnhancedActionEvents|EnhancedInputActionIA_OpenFolder
  (params (ActionValue :type Boolean) (ElapsedSeconds :type Float%20%28double-precision%29) (TriggeredSeconds :type Float%20%28double-precision%29) (InputAction :type Input%20Action%20Object%20Reference :default "/Game/Core/Inputs/IA_OpenFolder.IA_OpenFolder"))
  ;[1 1 1] Special interaction
  (:Started
    (bind _bestgrab (Default|CalculateCloserBestActor (Variables|Default|GetPlayerRef) "/Game/Blueprints/Props/BP_InteractiveProps.BP_InteractiveProps_C" (Variables|Default|GetRadius) -1.0))
    (Utilities|IsValid _bestgrab
      (:Is%20Valid
        (bind _asbp_interactive_props (Utilities|Casting|CastToBP_InteractiveProps _bestgrab))
        (Default|UpdateHistory (Variables|Default|GetMasterWidget) (Utilities|Text|ToText(String) (Utilities|String|Append "Interaction " (Utilities|String|ToString(Text) (Variables|/Game/Blueprints/Props/BP_InteractiveProps.BP_InteractiveProps_C|GetText _asbp_interactive_props)))))
        (Default|Interaction _asbp_interactive_props (Variables|Default|GetPlayerRef))))))

(event Input|EnhancedActionEvents|EnhancedInputActionIA_Grab
  (params (ActionValue :type Boolean) (ElapsedSeconds :type Float%20%28double-precision%29) (TriggeredSeconds :type Float%20%28double-precision%29) (InputAction :type Input%20Action%20Object%20Reference :default "/Game/Core/Inputs/IA_Grab.IA_Grab"))
  (bind _playerref (Variables|Default|GetPlayerRef))
  ;[1 1 1] Special interaction
  (:Started
    (Variables|/Game/Core/BP_Player.BP_Player_C|GetGrabbedComponent (Variables|Default|GetPlayerRef)
      (:then
        (Default|ReleaseComponent _playerref))
      (:else
        (Default|LaunchCable _playerref)))))

(event EventBeginPlay
  (bind _returnvalue (PlayerController|LocalPlayerSubsystems|GetEnhancedInputLocalPlayerSubsystem))
  ;[0.05098 0.05098 0.05098] Add Mapping Context
  (Utilities|IsValid _returnvalue
    (:Is%20Valid
      (Input|AddMappingContext _returnvalue (select (Utilities|Enum|NotEqual(Enum) (Utilities|Internationalization|GetCurrentCulture) "fr") "/Game/Core/Inputs/IMC_PlayerQwerty.IMC_PlayerQwerty" "/Game/Core/Inputs/IMC_PlayerAzerty.IMC_PlayerAzerty") 0 "(bIgnoreAllPressedKeysUntilRelease=True,bForceImmediately=False)")
      (Input|AddMappingContext _returnvalue "/Game/Core/Inputs/IMC_PlayerGamepad.IMC_PlayerGamepad" 0 "(bIgnoreAllPressedKeysUntilRelease=True,bForceImmediately=False)")
      (bind _returnvalue_2 (UserInterface|CreateWidget "/Game/UI/CUI_MasterWidget.CUI_MasterWidget_C" self))
      (bind _output_get (Variables|Default|SetMasterWidget _returnvalue_2))
      (UserInterface|Viewport|AddtoViewport _output_get 0)
      (bind _asbp_player (Utilities|Casting|CastToBP_Player (Pawn|GetControlledPawn)))
      (Variables|Default|SetPlayerRef _asbp_player))))

(fn ConstructionScript)