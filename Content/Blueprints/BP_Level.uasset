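; BP_Level is a container actor that groups a list of props so they can be shown or hidden together as a level chunk.
; The construction script attaches each listed prop to it, keeping world transforms.
; UpdateVisibility stores the Loaded flag and propagates visibility from the root through the attached hierarchy.
; On BeginPlay it applies that flag and, if PhysicOn is false, disables physics simulation on movable props.
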(event Custom|DeactivateChildPhysics
  (for _array_element (Variables|Default|GetListChildProps)
    (if (Variables|/Game/Blueprints/Props/BP_Props.BP_Props_C|GetCanMove _array_element)
      (Physics|SetSimulatePhysics (Variables|/Game/Blueprints/Props/BP_Props.BP_Props_C|GetStaticMesh _array_element) false))))

(event EventBeginPlay
  (Utilities|FlowControl|Sequence
    (:then_0
      (CallFunction|UpdateVisibility (Variables|Default|GetLoaded)))
    (:then_1
      (if (not (Variables|Default|GetbPhysicOn))
        (CallFunction|DeactivateChildPhysics)))))

(fn ConstructionScript
  (CallFunction|AttachObject))

(fn AttachObject
  (for _array_element (Variables|Default|GetListChildProps)
    (Transformation|AttachActorToActor _array_element self "None" "KeepWorld" "KeepWorld" "KeepWorld" true)))

(fn UpdateVisibility
  (params (Loaded :type Boolean))
  (Variables|Default|SetLoaded Loaded)
  (Rendering|SetVisibility (Variables|Default|GetDefaultSceneRoot) (Variables|Default|GetLoaded) true))