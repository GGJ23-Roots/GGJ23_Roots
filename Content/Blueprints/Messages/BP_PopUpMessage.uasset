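; BP_PopUpMessage is a world-placed actor that shows a pop-up message when the player comes within a set display distance.
; On BeginPlay it copies its title and content into the UI_PopUp_Message widget of its widget component and caches the BP_Player actor.
; A looping half-second timer compares the distance to the player against DisplayDistance and toggles the widget component's visibility, avoiding per-tick checks.
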(event Custom|EvaluateDistanceToPlayer
  (bind _playerref (Variables|Default|GetPlayerRef)
    (:then
      (bind _output_get (Variables|Default|SetDistanceFromPlayer (Math|Vector|Distance(Vector) (Transformation|GetActorLocation) (Transformation|GetActorLocation _playerref))))
      (if (<= _output_get (Variables|Default|GetDisplayDistance))
        (CallFunction|DisplayMessage)
        (else
          (CallFunction|HideMesssage))))
    (:else)))

(event Custom|HideMesssage
  (Rendering|SetVisibility (Variables|Default|GetWidget) false false))

(event Custom|DisplayMessage
  (Rendering|SetVisibility (Variables|Default|GetWidget) true false))

(event EventBeginPlay
  (bind _asui_pop_up_message (Utilities|Casting|CastToUI_PopUp_Message (UserInterface|GetWidget (Variables|Default|GetWidget))))
  (Variables|/Game/UI/UI_PopUp_Message.UI_PopUp_Message_C|SetMessageTitle _asui_pop_up_message (Variables|Default|GetMessageTitle))
  (Variables|/Game/UI/UI_PopUp_Message.UI_PopUp_Message_C|SetMessageContent _asui_pop_up_message (Variables|Default|GetMessageContent))
  (bind _returnvalue (Actor|GetActorOfClass "/Game/Core/BP_Player.BP_Player_C"))
  (Variables|Default|SetPlayerRef _returnvalue)
  (Utilities|Time|SetTimerbyEvent (delegate Custom|EvaluateDistanceToPlayer) 0.5 true))

(fn ConstructionScript)