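; BP_Pong is a self-contained Pong minigame actor where the player plays an AI to three points.
; A physics ball launches by random diagonal impulse, and goal overlaps score, then either relaunch it after a delay or end the game with debug prints.
; Each Tick, the left AI racket chases the ball without delta-time scaling, clamped to its track, while the right racket's position follows a debug mouse-axis value.
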(event OnComponentBeginOverlap(LeftGoal)
  (params (OverlappedComponent :type Primitive%20Component%20Object%20Reference) (OtherActor :type Actor%20Object%20Reference) (OtherComp :type Primitive%20Component%20Object%20Reference) (OtherBodyIndex :type Integer) (bFromSweep :type Boolean) (SweepResult :type Hit%20Result%20Structure%20%28by%20ref%29))
  (bind _playerpoints (Variables|Default|GetPlayerPoints))
  ;[1 1 1] Point scoring and endgame
  (if (== OtherComp (Variables|Default|GetBall))
    (Math|Integer|IncrementInt _playerpoints
      (:%20%20
        (if (>= _playerpoints 3)
          (CallFunction|EndGame true)
          (else
            (CallFunction|ResetBall)
            (Utilities|FlowControl|Delay 2.0)
            (CallFunction|LaunchBall)))))))

(event OnComponentBeginOverlap(RightGoal)
  (params (OverlappedComponent :type Primitive%20Component%20Object%20Reference) (OtherActor :type Actor%20Object%20Reference) (OtherComp :type Primitive%20Component%20Object%20Reference) (OtherBodyIndex :type Integer) (bFromSweep :type Boolean) (SweepResult :type Hit%20Result%20Structure%20%28by%20ref%29))
  (bind _iapoints (Variables|Default|GetIAPoints))
  ;[1 1 1] Point scoring and endgame
  (if (== OtherComp (Variables|Default|GetBall))
    (Math|Integer|IncrementInt _iapoints
      (:%20%20
        (if (>= _iapoints 3)
          (CallFunction|EndGame false)
          (else
            (CallFunction|ResetBall)
            (Utilities|FlowControl|Delay 2.0)
            (CallFunction|LaunchBall)))))))

(event EventBeginPlay
  ;[1 1 1] Start game Debug
  (CallFunction|LaunchBall)
  (Input|EnableInput (Game|GetPlayerController 0)))

(event EventTick
  (params (DeltaSeconds :type Float%20%28single-precision%29))
  (bind _ball (Variables|Default|GetBall))
  (bind _leftracket (Variables|Default|GetLeftRacket))
  (bind _returnvalue (Transformation|GetWorldLocation _ball))
  (bind _returnvalue_2 (Transformation|GetWorldLocation _leftracket))
  (bind _returnvalue_3 (- _returnvalue _returnvalue_2))
  ;[1 1 1] IA (testing if currently winnable)
  (Transformation|AddWorldOffset _leftracket (* (/ _returnvalue_3 (Math|Vector|VectorLength _returnvalue_3)) (Variables|Default|GetRacketsSpeed)) false false)
  (Transformation|SetRelativeLocation _leftracket (Math|Vector|MakeVector -75.0 (Math|Float|Clamp(Float) (.y (Variables|/Script/Engine.SceneComponent|GetRelativeLocation _leftracket)) -4e+01 4e+01) 5.0) false false)
  (CallFunction|MovePlayerRacket (Variables|Default|GetDebugMovement)))

(event Input|AxisEvents|InputAxisLookUp/DownMouse
  (params (AxisValue :type Float%20%28single-precision%29))
  ;[1 1 1] Start game Debug
  (bind _output_get (Variables|Default|SetDebugMovement AxisValue))
  (Development|PrintString (Utilities|String|ToString(Float) _output_get)))

(fn ConstructionScript)

(fn MovePlayerRacket
  (params (Location :type Float%20%28double-precision%29))
  (bind _rightracket (Variables|Default|GetRightRacket))
  (bind _relativelocation (Variables|/Script/Engine.SceneComponent|GetRelativeLocation _rightracket))
  (Transformation|SetRelativeLocation _rightracket (Math|Vector|MakeVector (.x _relativelocation) (* (Math|Float|Clamp(Float) Location -1.0) 4e+01) (.z _relativelocation)) false false))

(fn LaunchBall
  (if (Math|Random|RandomBool)
    (bind _output_get (LocalVariables|SetDirection (Math|Vector|MakeVector 0.0 1.0 0.0)))
    (else
      (bind _output_get_2 (LocalVariables|SetDirection (Math|Vector|MakeVector 0.0 -1.0 0.0)))))
  (if (Math|Random|RandomBool)
    (LocalVariables|SetDirection (Math|Vector|MakeVector (Math|Random|RandomFloatinRange 0.25 1.0) (.y _output_get) (.z _output_get)))
    (else
      (LocalVariables|SetDirection (Math|Vector|MakeVector (Math|Random|RandomFloatinRange -1.0 -0.25) (.y _output_get_2) (.z _output_get_2)))))
  (Physics|AddImpulse (Variables|Default|GetBall) (* (Math|Vector|Normalize (LocalVariables|GetDirection)) (Variables|Default|GetBallSpeed)) "None" true))

(fn StartGame
  (Variables|Default|SetPlayerPoints 0)
  (Variables|Default|SetIAPoints 0)
  (CallFunction|LaunchBall))

(fn ResetBall
  (bind _ball (Variables|Default|GetBall))
  (Transformation|SetWorldLocation _ball (Transformation|GetWorldLocation (Variables|Default|GetDefaultSceneRoot)) false false)
  (Physics|SetPhysicsLinearVelocity _ball "0, 0, 0" false "None"))

(fn EndGame
  (params (PlayerWon :type Boolean))
  (Development|PrintString "Pong game has ended")
  (if PlayerWon
    (Development|PrintString "Player has won")
    (else
      (Development|PrintString "IA has won")))
  (CallFunction|ResetBall))