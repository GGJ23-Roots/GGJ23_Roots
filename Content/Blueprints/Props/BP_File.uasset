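; BP_File is a physical desktop-file prop with a mesh chosen by folder type and a popup name label.
; Mass and width derive from the image's texture memory unless overridden.
; Opening it spawns an image widget that flies onto the desktop background at a random spot, or onto BP_Pong to reveal it, then the file destroys itself.
; Fast overlaps play speed-tiered hit sounds and damage BP_Bug while the file is grabbed.
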(event OnComponentBeginOverlap(Box)
  (params (OverlappedComponent :type Primitive%20Component%20Object%20Reference) (OtherActor :type Actor%20Object%20Reference) (OtherComp :type Primitive%20Component%20Object%20Reference) (OtherBodyIndex :type Integer) (bFromSweep :type Boolean) (SweepResult :type Hit%20Result%20Structure%20%28by%20ref%29))
  (bind _returnvalue (Transformation|GetVelocity))
  (bind _returnvalue_2 (Transformation|GetActorLocation))
  (Utilities|FlowControl|Sequence
    (:then_0
      (bind _asbp_bug (Utilities|Casting|CastToBP_Bug OtherActor))
      (Variables|Default|GetGrabbedBy
        (:then
          (if (> (Math|Vector|VectorLength (Transformation|GetVelocity)) 3e+02)
            (Default|TakeDamage _asbp_bug)))
        (:else)))
    (:then_1
      (if (>= (Math|Vector|VectorLength _returnvalue) (Variables|Default|GetHeavyHitThreashold))
        (Audio|PlaySoundatLocation "/Game/Audio/SFX/File_Hit/SFX_File_Hit_Heavy.SFX_File_Hit_Heavy" _returnvalue_2 "0, 0, 0" 1.0 1.0 0.0 0 0 0 0)
        (elif (>= (Math|Vector|VectorLength _returnvalue) (Variables|Default|GetMediumHitThreshold))
          (Audio|PlaySoundatLocation "/Game/Audio/SFX/File_Hit/SFX_File_Hit_Medium.SFX_File_Hit_Medium" _returnvalue_2 "0, 0, 0" 1.0 1.0 0.0 0 0 0 0)
          (elif (>= (Math|Vector|VectorLength _returnvalue) (Variables|Default|GetLightHitThreshold))
            (Audio|PlaySoundatLocation "/Game/Audio/SFX/File_Hit/SFX_File_Hit_Light.SFX_File_Hit_Light" _returnvalue_2 "0, 0, 0" 1.0 1.0 0.0 0 0 0 0)))))))

(event EventBeginPlay
  (|CallParentFunction)
  (bind _astexture_2d (Utilities|Casting|CastToTexture2D (Class|WidgetBlueprintLibrary|GetBrushResource (Variables|Default|GetBrush%20File))))
  (Class|PrimitiveComponent|SetMassOverrideinKg (Variables|Default|GetStaticMesh) "None" (select (Variables|Default|GetOverrideMass) (Variables|Default|GetWeight) (Math|Float|Clamp(Float) (Math|Conversions|ToFloat(Integer) (/ (Class|Texture|BlueprintGetMemorySize _astexture_2d) 100000)) 1e+01 2e+02)) true)
  (Transformation|SetWorldScale3D (Variables|Default|GetStaticMesh) (Math|Vector|MakeVector 1.0 (Math|Float|MapRangeClamped (select (Variables|Default|GetOverrideMass) (Variables|Default|GetWeight) (Math|Float|Clamp(Float) (Math|Conversions|ToFloat(Integer) (/ (Class|Texture|BlueprintGetMemorySize _astexture_2d) 100000)) 1e+01 2e+02)) 1e+01 1e+02 0.4 1.0) 1.0))
  (bind _asui_pop_name (Utilities|Casting|CastToUI_PopName (UserInterface|GetWidget (Variables|Default|GetWidget))))
  (if (Variables|Default|GetbOverrideByImageName)
    (Variables|Default|SetText (Utilities|Text|ToText(String) (Utilities|GetDisplayName (.ResourceObject (Utilities|Struct|BreakSlateBrush (Variables|Default|GetBrush%20File)))))))
  (Default|SetTextFolderFile _asui_pop_name (Utilities|Text|ToText(String) (Utilities|String|Append (Utilities|String|ToString(Text) (Variables|Default|GetText)) (Variables|Default|GetExtension)))))

(event EventActionZone
  (params (ActionZoneType :type E_ActionZoneType%20Enum :default "NewEnumerator0"))
  (switch Utilities|FlowControl|Switch|SwitchonE_ActionZoneType ActionZoneType
    (:NewEnumerator0
      (Audio|Components|Audio|Play (Variables|Default|GetAudio) 0.0)
      (bind _returnvalue (Game|SpawnActorfromClass "/Game/BP_FileWidgetOpen.BP_FileWidgetOpen_C" (Math|Transform|MakeTransform (+ (Transformation|GetActorLocation) "0.000000,0.000000,150.000000") "0, 0, 0" "1.000000,1.000000,1.000000") "Undefined" 0 (Variables|Default|GetBrush%20File) 0))
      (Variables|Default|SetFileWidget _returnvalue)
      (if (Variables|Default|GetPong?)
        (bind _returnvalue_2 (Actor|GetActorOfClass "/Game/Blueprints/Pong/BP_Pong.BP_Pong_C"))
        (bind _output_get (Variables|Default|SetPong _returnvalue_2))
        (Utilities|IsValid _output_get
          (:Is%20Valid
            _))
        (else
          (bind _returnvalue_3 (Actor|GetActorOfClass "/Game/Blueprints/Props/WorldWidgets/BP_DesktopWorldWIdget.BP_DesktopWorldWIdget_C"))
          (bind _output_get_2 (Variables|Default|SetBackground _returnvalue_3))
          (Utilities|IsValid _output_get_2
            (:Is%20Valid
              _))))
      (Utilities|FlowControl|Delay (Variables|Default|GetTimeBeforeMoveOnBG))
      (Components|Activation|Deactivate (Variables|/Game/BP_FileWidgetOpen.BP_FileWidgetOpen_C|GetRotatingMovement (Variables|Default|GetFileWidget)))
      (Variables|Default|SetOldTransform (Transformation|GetActorTransform (Variables|Default|GetFileWidget)))
      (if (Variables|Default|GetPong?)
        (bind _newtrack_0 (Timeline|Timeline PlayFromStart)
          (:Update
            (Transformation|SetActorTransform (Variables|Default|GetFileWidget) (Math|Transform|MakeTransform (.location (Math|Transform|Lerp(Transform) (Variables|Default|GetOldTransform) (Math|Transform|MakeTransform (Math|Vector|MakeVector (+ (.x (.location (Transformation|GetActorTransform (select (Variables|Default|GetPong?) (Variables|Default|GetPong) (Variables|Default|GetBackground))))) -1e+01) (+ (.y (.location (Transformation|GetActorTransform (select (Variables|Default|GetPong?) (Variables|Default|GetPong) (Variables|Default|GetBackground))))) (Variables|Default|GetBackgroundRandomY)) (+ (.z (.location (Transformation|GetActorTransform (select (Variables|Default|GetPong?) (Variables|Default|GetPong) (Variables|Default|GetBackground))))) (Variables|Default|GetBackgroundRandomZ))) (.rotation (Transformation|GetActorTransform (select (Variables|Default|GetPong?) (Variables|Default|GetPong) (Variables|Default|GetBackground)))) (Variables|Default|GetOnScreenFinalScale)) _newtrack_0)) (.rotation (Math|Transform|Lerp(Transform) (Variables|Default|GetOldTransform) (Math|Transform|MakeTransform (Math|Vector|MakeVector (+ (.x (.location (Transformation|GetActorTransform (select (Variables|Default|GetPong?) (Variables|Default|GetPong) (Variables|Default|GetBackground))))) -1e+01) (+ (.y (.location (Transformation|GetActorTransform (select (Variables|Default|GetPong?) (Variables|Default|GetPong) (Variables|Default|GetBackground))))) (Variables|Default|GetBackgroundRandomY)) (+ (.z (.location (Transformation|GetActorTransform (select (Variables|Default|GetPong?) (Variables|Default|GetPong) (Variables|Default|GetBackground))))) (Variables|Default|GetBackgroundRandomZ))) (.rotation (Transformation|GetActorTransform (select (Variables|Default|GetPong?) (Variables|Default|GetPong) (Variables|Default|GetBackground)))) (Variables|Default|GetOnScreenFinalScale)) _newtrack_0)) (.scale (Math|Transform|Lerp(Transform) (Variables|Default|GetOldTransform) (Math|Transform|MakeTransform (Math|Vector|MakeVector (+ (.x (.location (Transformation|GetActorTransform (select (Variables|Default|GetPong?) (Variables|Default|GetPong) (Variables|Default|GetBackground))))) -1e+01) (+ (.y (.location (Transformation|GetActorTransform (select (Variables|Default|GetPong?) (Variables|Default|GetPong) (Variables|Default|GetBackground))))) (Variables|Default|GetBackgroundRandomY)) (+ (.z (.location (Transformation|GetActorTransform (select (Variables|Default|GetPong?) (Variables|Default|GetPong) (Variables|Default|GetBackground))))) (Variables|Default|GetBackgroundRandomZ))) (.rotation (Transformation|GetActorTransform (select (Variables|Default|GetPong?) (Variables|Default|GetPong) (Variables|Default|GetBackground)))) (Variables|Default|GetOnScreenFinalScale)) _newtrack_0))) false true))
          (:Finished
            (Audio|Components|Audio|FadeOut (Variables|Default|GetAudio) 0.5 0.0 "Linear" :!class /Script/Engine.AudioComponent)
            (if (Variables|Default|GetPong?)
              (Rendering|SetActorHiddenInGame (Variables|Default|GetPong) false)
              (Actor|DestroyActor (Variables|Default|GetFileWidget))
              (Actor|DestroyActor)
              (else
                (Transformation|AttachActorToActor (Variables|Default|GetFileWidget) (Variables|Default|GetBackground) "None" "KeepWorld" "KeepWorld" "KeepWorld" true)
                (Actor|SetLifeSpan (Variables|Default|GetFileWidget) (Variables|Default|GetFileDestroyTimer))
                (Actor|DestroyActor)))))
        (else
          (Variables|Default|SetBackgroundRandomY (Math|Random|RandomIntegerinRange -750 750))
          (Variables|Default|SetBackgroundRandomZ (Math|Random|RandomIntegerinRange -220 310))
          (Timeline|Timeline PlayFromStart))))))

(event EventPopUpText
  (params (Animation :type EUMGSequencePlayMode%20Enum :default "Forward"))
  (bind _asui_pop_name (Utilities|Casting|CastToUI_PopName (UserInterface|GetWidget (Variables|Default|GetWidget))))
  (Default|TextAnimation _asui_pop_name Animation))

(fn ConstructionScript
  (bind _staticmesh (Variables|Default|GetStaticMesh))
  (|CallParentFunction)
  (bind _returnvalue (Rendering|Material|CreateDynamicMaterialInstance _staticmesh 0 "/Game/StaticMeshes/Global/M_Props_Palet3.M_Props_Palet3" "None" :!class /Script/Engine.PrimitiveComponent))
  (Components|StaticMesh|SetStaticMesh _staticmesh (Utilities|Select :Index (Variables|Default|GetFolderType) :NewEnumerator0 "/Game/StaticMeshes/Folders/Antivirus/GGJ23-Props-Folders-Antivirus.GGJ23-Props-Folders-Antivirus" :NewEnumerator1 "/Game/StaticMeshes/Folders/Game/GGJ23-Props-Folders-Game.GGJ23-Props-Folders-Game" :NewEnumerator2 "/Game/StaticMeshes/Folders/Image/GGJ23-Props-Folders-Image.GGJ23-Props-Folders-Image" :NewEnumerator3 "/Game/StaticMeshes/Folders/Video/GGJ23-Props-Folders-Video.GGJ23-Props-Folders-Video"))
  (Rendering|Material|SetMaterial _staticmesh 0 _returnvalue))