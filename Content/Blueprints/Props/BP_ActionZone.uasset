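; BP_ActionZone is a trigger zone that runs an Open, Duplicate or Delete action on a BP_InteractiveProps "file" entering its box.
; Overlap links one prop and starts a delayed timer for the zone's action type; leaving unlinks it unless an action is in progress.
; Open releases the prop, slides it horizontally via timeline, then calls its ActionZone.
; Delete plays a sound, releases the player's grab and destroys it; Duplicate is an empty stub.
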(event OnComponentBeginOverlap(Box)
  (params (OverlappedComponent :type Primitive%20Component%20Object%20Reference) (OtherActor :type Actor%20Object%20Reference) (OtherComp :type Primitive%20Component%20Object%20Reference) (OtherBodyIndex :type Integer) (bFromSweep :type Boolean) (SweepResult :type Hit%20Result%20Structure%20%28by%20ref%29))
  (Variables|Default|GetLinkedProps
    (:then)
    (:else
      (bind _asbp_interactive_props (Utilities|Casting|CastToBP_InteractiveProps OtherActor))
      (Variables|Default|SetLinkedProps _asbp_interactive_props)
      (CallFunction|ActionZone (Variables|Default|GetActionType)))))

(event OnComponentEndOverlap(Box)
  (params (OverlappedComponent :type Primitive%20Component%20Object%20Reference) (OtherActor :type Actor%20Object%20Reference) (OtherComp :type Primitive%20Component%20Object%20Reference) (OtherBodyIndex :type Integer))
  (bind _asbp_interactive_props (Utilities|Casting|CastToBP_InteractiveProps OtherActor))
  (if (and (== _asbp_interactive_props (Variables|Default|GetLinkedProps)) (not (Variables|Default|GetActionInProgress)))
    (Variables|Default|SetLinkedProps 0)))

(event Custom|OpenAction
  (bind _returnvalue (Transformation|GetActorLocation))
  (bind _openfolderlocation (Variables|Default|GetOpenFolderLocation))
  (bind _returnvalue_2 (+ _returnvalue _openfolderlocation))
  (bind _linkedprops (Variables|Default|GetLinkedProps)
    (:then
      (Default|ReleaseComponent (Variables|/Game/Blueprints/Props/BP_InteractiveProps.BP_InteractiveProps_C|GetGrabbedBy _linkedprops))
      (Variables|/Game/Blueprints/Props/BP_InteractiveProps.BP_InteractiveProps_C|SetGrabbedBy _linkedprops (Variables|/Game/Blueprints/Props/BP_InteractiveProps.BP_InteractiveProps_C|GetGrabbedBy _linkedprops))
      (Variables|Default|SetStartLerp (Transformation|GetActorLocation _linkedprops))
      (Variables|/Game/Blueprints/Props/BP_Props.BP_Props_C|SetCanMove (Variables|Default|GetLinkedProps) false)
      (Default|UpdateCanMove (Variables|Default|GetLinkedProps))
      (Variables|Default|SetActionInProgress true)
      (bind _newtrack_0 (Timeline|Timeline PlayFromStart)
        (:Update
          (bind _linkedprops_2 (Variables|Default|GetLinkedProps)
            (:then
              (Transformation|SetActorLocation _linkedprops_2 (Math|Vector|Lerp(Vector) (Variables|Default|GetStartLerp) (Math|Vector|MakeVector (.x _returnvalue_2) (.y _returnvalue_2) (.Z (Class|KismetMathLibrary|BreakVector3f (Variables|Default|GetStartLerp)))) _newtrack_0) false true))
            (:else)))
        (:Finished
          ;[1 1 1] timeline finish :  add pop up open file in the background
          (Variables|Default|SetActionInProgress false)
          (Variables|/Game/Blueprints/Props/BP_Props.BP_Props_C|SetCanMove (Variables|Default|GetLinkedProps) true)
          (Default|ActionZone (Variables|Default|GetLinkedProps) (Variables|Default|GetActionType))
          (Variables|Default|SetLinkedProps 0))))
    (:else)))

(event EventActionZone
  (params (ActionZoneType :type E_ActionZoneType%20Enum :default "NewEnumerator0"))
  (if (not (Variables|Default|GetActionInProgress))
    (switch Utilities|FlowControl|Switch|SwitchonE_ActionZoneType ActionZoneType
      (:NewEnumerator0
        (Utilities|Time|SetTimerbyEvent (delegate Custom|OpenAction) (Variables|Default|GetOpenTime)))
      (:NewEnumerator1
        (Utilities|Time|SetTimerbyFunctionName 0 "DuplicateFile" (Variables|Default|GetDuplicateTime)))
      (:NewEnumerator2
        (Utilities|Time|SetTimerbyFunctionName 0 "DeleteFile" (Variables|Default|GetDeleteTime))))))

(fn ConstructionScript
  (|CallParentFunction))

(fn DuplicateFile)

(fn DeleteFile
  (bind _linkedprops (Variables|Default|GetLinkedProps)
    (:then
      (Audio|PlaySound2D "/Game/Audio/SFX/File/SC_File_Destroy.SC_File_Destroy" 1.0 1.0 0.0 0 0)
      (Default|ReleaseComponent (.AsBP%20Player (Utilities|Casting|CastToBP_Player (Game|GetPlayerCharacter 0))))
      (Actor|DestroyActor _linkedprops)
      (Variables|Default|SetLinkedProps 0))
    (:else)))