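; World-space desktop widget actor that trails the player and hosts the UI_DesktopWidget pause menu.
; OpenMenuPause passes the owning player to the widget, then opens its pause menu.
; BeginPlay caches BP_Player, and Tick slowly interpolates toward its location with Y and Z offsets.
; Each interpolation step restarts X from BaseX, so the actor stays near that depth while easing along Y and Z.
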(event Custom|OpenMenuPause
  (params (OwningPlayer :type Player%20Controller%20Object%20Reference))
  (bind _asui_desktop_widget (Utilities|Casting|CastToUI_DesktopWidget (UserInterface|GetWidget (Variables|Default|GetWidget))))
  (Class|UserWidget|SetOwningPlayer _asui_desktop_widget OwningPlayer)
  (Default|OpenMenuPause _asui_desktop_widget))

(event EventBeginPlay
  (bind _returnvalue (Actor|GetActorOfClass "/Game/Core/BP_Player.BP_Player_C"))
  (Variables|Default|SetBP_Player _returnvalue))

(event EventTick
  (params (DeltaSeconds :type Float%20%28single-precision%29))
  (bind _returnvalue (Transformation|GetActorLocation))
  (bind _bp_player (Variables|Default|GetBP_Player))
  (bind _returnvalue_2 (Transformation|GetActorLocation _bp_player))
  (Transformation|SetActorLocation (Math|Interpolation|VInterpTo (Math|Vector|MakeVector (Variables|Default|GetBaseX) (.y _returnvalue) (.z _returnvalue)) (Math|Vector|MakeVector (.x _returnvalue_2) (+ (.y _returnvalue_2) (Variables|Default|GetOffsetY)) (+ (.z _returnvalue_2) (Variables|Default|GetOffsetZ))) DeltaSeconds 0.7) false false))

(fn ConstructionScript)