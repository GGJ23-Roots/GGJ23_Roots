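; BP_Bit is a randomly scaled moving hazard that knocks props and players away on contact.
; A looping timer steps it along its forward vector with a swept move.
; On mesh overlap it launches a BP_Props after calling ReleaseComponent on the player, or shoves an un-hit BP_Player's physics-enabled capsule at a slightly random angle and calls GetBackUp.
; It destroys itself after any such overlap, whatever it touched.
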(event OnComponentBeginOverlap(StaticMesh)
  (params (OverlappedComponent :type Primitive%20Component%20Object%20Reference) (OtherActor :type Actor%20Object%20Reference) (OtherComp :type Primitive%20Component%20Object%20Reference) (OtherBodyIndex :type Integer) (bFromSweep :type Boolean) (SweepResult :type Hit%20Result%20Structure%20%28by%20ref%29))
  (Utilities|FlowControl|Sequence
    (:then_0
      (bind _asbp_props (Utilities|Casting|CastToBP_Props OtherActor))
      (Default|ReleaseComponent (Variables|Default|GetPlayerRef))
      (Physics|AddImpulse (Variables|/Game/Blueprints/Props/BP_Props.BP_Props_C|GetStaticMesh _asbp_props) (* (Transformation|GetActorForwardVector) (Variables|Default|GetImpulsePower)) "None" true))
    (:then_1
      (bind _asbp_player (Utilities|Casting|CastToBP_Player OtherActor))
      (if (not (Variables|/Game/Core/BP_Player.BP_Player_C|GetHit _asbp_player))
        (Physics|SetSimulatePhysics (Variables|/Script/Engine.Character|GetCapsuleComponent _asbp_player) true)
        (Physics|AddImpulse (Variables|/Script/Engine.Character|GetCapsuleComponent _asbp_player) (* (Math|Vector|RotateVectorAroundAxis (Transformation|GetActorForwardVector) (Math|Random|RandomFloatinRange -1e+01 1e+01) "0.000000,0.000000,1.000000") (Variables|Default|GetImpulsePower)) "None" true)
        (Default|GetBackUp _asbp_player)))
    (:then_2
      (Actor|DestroyActor))))

(event Custom|Movement
  (Transformation|SetActorLocation (+ (Transformation|GetActorLocation) (* (Transformation|GetActorForwardVector) (Variables|Default|GetDistanceTick))) true false))

(event EventBeginPlay
  (bind _asbp_player (Utilities|Casting|CastToBP_Player (Game|GetPlayerCharacter 0)))
  (Variables|Default|SetPlayerRef _asbp_player)
  (Transformation|SetWorldScale3D (Variables|Default|GetStaticMesh) (Math|Conversions|ToVector(Float) (Math|Random|RandomFloatinRange 0.8 1.2)))
  (Utilities|Time|SetTimerbyEvent (delegate Custom|Movement) (Variables|Default|GetSpeedTick) true))

(event Collision|EventActorBeginOverlap
  (params (OtherActor :type Actor%20Object%20Reference)))

(event EventTick
  (params (DeltaSeconds :type Float%20%28single-precision%29)))

(fn ConstructionScript)