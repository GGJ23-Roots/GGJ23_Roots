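; Computer file prop, a child of a folder-type Blueprint, that represents a random PNG from the player's own Pictures folder.
; On BeginPlay it derives that path from the user directory, picks a recursively found PNG, imports it at runtime and stores it as a brush.
; After the parent BeginPlay, it shows the cleaned filename on its UI_PopName widget.
; The construction script forces the inherited FolderType to a fixed enum value.
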(event EventBeginPlay
  (bind _returnvalue (Class|BlueprintFileUtilsBPLibrary|GetUserDirectory))
  (bind _foundpaths (Class|BlueprintFileUtilsBPLibrary|FindRecursive (Utilities|String|Append (Utilities|String|GetSubstring _returnvalue 0 (+ (Utilities|String|FindSubstring _returnvalue "/" false true (- (Utilities|String|Len _returnvalue) 1)) 1)) "Pictures/") "*.png" true false))
  (bind _output_get (Variables|Default|SetFile (.OutItem (Utilities|Array|Random _foundpaths))))
  (bind _returnvalue_2 (Class|KismetRenderingLibrary|ImportFileasTexture2D _output_get))
  (Variables|Default|SetBrush%20File (Class|WidgetBlueprintLibrary|MakeBrushfromTexture _returnvalue_2))
  (|CallParentFunction)
  (bind _asui_pop_name (Utilities|Casting|CastToUI_PopName (UserInterface|GetWidget (Variables|Default|GetWidget))))
  (Default|SetTextFolderFile _asui_pop_name (Utilities|Text|ToText(String) (Class|BlueprintPathsLibrary|GetCleanFilename (Variables|Default|GetFile)))))

(event Collision|EventActorBeginOverlap
  (params (OtherActor :type Actor%20Object%20Reference))
  (|CallParentFunction OtherActor) ; This node is disabled and will not be called.\nDrag off pins to build functionality.
)

(event EventTick
  (params (DeltaSeconds :type Float%20%28single-precision%29))
  (|CallParentFunction DeltaSeconds) ; This node is disabled and will not be called.\nDrag off pins to build functionality.
)

(fn ConstructionScript
  (if (Utilities|Enum|NotEqual(Enum) (Variables|Default|GetFolderType) "NewEnumerator2")
    (Variables|Default|SetFolderType "NewEnumerator2"))
  (|CallParentFunction))