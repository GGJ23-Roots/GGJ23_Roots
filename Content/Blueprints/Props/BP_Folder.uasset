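; BP_Folder is an interactable folder prop that teleports the player to its TargetLevel actor when used.
; EnterFolder moves any grabbed component and the player to the target, updates the player's CurrentLevel and reverses the name popup animation.
; The construction script picks the mesh by FolderType and applies a dynamic palette material.
; A UI_PopName widget shows the folder's text, set on BeginPlay and animated through PopUpText.
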(event EventBeginPlay
  (|CallParentFunction)
  (bind _asui_pop_name (Utilities|Casting|CastToUI_PopName (UserInterface|GetWidget (Variables|Default|GetWidget))))
  (Default|SetTextFolderFile _asui_pop_name (Variables|Default|GetText)))

(event Collision|EventActorBeginOverlap
  (params (OtherActor :type Actor%20Object%20Reference)))

(event EventTick
  (params (DeltaSeconds :type Float%20%28single-precision%29)))

(event EventInteraction
  (params (Player :type BP%20Player%20Object%20Reference))
  (CallFunction|EnterFolder Player))

(event EventActionZone
  (params (ActionZoneType :type E_ActionZoneType%20Enum :default "NewEnumerator0"))
  (switch Utilities|FlowControl|Switch|SwitchonE_ActionZoneType ActionZoneType))

(event EventPopUpText
  (params (Animation :type EUMGSequencePlayMode%20Enum :default "Forward"))
  (bind _asui_pop_name (Utilities|Casting|CastToUI_PopName (UserInterface|GetWidget (Variables|Default|GetWidget))))
  (Default|TextAnimation _asui_pop_name Animation))

(fn ConstructionScript
  (bind _staticmesh (Variables|Default|GetStaticMesh))
  (|CallParentFunction)
  (bind _returnvalue (Rendering|Material|CreateDynamicMaterialInstance _staticmesh 0 "/Game/StaticMeshes/Global/M_Props_Palet3.M_Props_Palet3" "None" :!class /Script/Engine.PrimitiveComponent))
  (Components|StaticMesh|SetStaticMesh _staticmesh (Utilities|Select :Index (Variables|Default|GetFolderType) :NewEnumerator0 "/Game/StaticMeshes/Folders/Antivirus/GGJ23-Props-Folders-Antivirus.GGJ23-Props-Folders-Antivirus" :NewEnumerator1 "/Game/StaticMeshes/Folders/Game/GGJ23-Props-Folders-Game.GGJ23-Props-Folders-Game" :NewEnumerator2 "/Game/StaticMeshes/Folders/Image/GGJ23-Props-Folders-Image.GGJ23-Props-Folders-Image" :NewEnumerator3 "/Game/StaticMeshes/Folders/Video/GGJ23-Props-Folders-Video.GGJ23-Props-Folders-Video"))
  (Rendering|Material|SetMaterial _staticmesh 0 _returnvalue))

(fn EnterFolder
  (params (Player :type BP%20Player%20Object%20Reference))
  (bind _targetlevel (Variables|Default|GetTargetLevel))
  (bind _grabbedcomponent (Variables|/Game/Core/BP_Player.BP_Player_C|GetGrabbedComponent Player))
  (bind _returnvalue (Transformation|GetActorTransform _targetlevel))
  (Utilities|IsValid _grabbedcomponent
    (:Is%20Valid
      (Transformation|SetWorldLocation _grabbedcomponent (.Location (Math|Transform|BreakTransform _returnvalue)) false true))
    (:Is%20Not%20Valid
      _))
  (Transformation|SetActorTransform Player _returnvalue false true)
  (bind _output_get (Variables|/Game/Core/BP_Player.BP_Player_C|SetCurrentLevel Player (Variables|Default|GetTargetLevel)))
  (CallFunction|PopUpText "Reverse"))