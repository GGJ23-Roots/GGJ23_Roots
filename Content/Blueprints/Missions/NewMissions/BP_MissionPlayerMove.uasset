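; Mission Blueprint that tasks the player with moving to a Destination actor.
; Each Tick, until MissionDone, it pushes the title, text and progress to the UI_PopUp_Mission widget inside the BP_MissionPopUp actor.
; Progress is MaxDistance divided by the current player-to-Destination distance, clamped to 0–1, so EndMission fires once the player is within MaxDistance.
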(event EventTick
  (params (DeltaSeconds :type Float%20%28single-precision%29))
  (|CallParentFunction 0.0)
  (if (not (Variables|Default|GetMissionDone))
    (bind _player (Variables|Default|GetPlayer)
      (:then
        (bind _asbp_mission_pop_up (Utilities|Casting|CastToBP_MissionPopUp (Variables|Default|GetMissionPopup)))
        (bind _asui_pop_up_mission (Utilities|Casting|CastToUI_PopUp_Mission (UserInterface|GetUserWidgetObject (Variables|/Game/Blueprints/Missions/NewMissions/BP_MissionPopUp.BP_MissionPopUp_C|GetMissionWidget _asbp_mission_pop_up))))
        (Variables|/Game/UI/UI_PopUp_Mission.UI_PopUp_Mission_C|SetMissionTitle _asui_pop_up_mission (Variables|Default|GetMissionTitle))
        (Variables|/Game/UI/UI_PopUp_Mission.UI_PopUp_Mission_C|SetMissionProgressText _asui_pop_up_mission (Variables|Default|GetMissionText))
        (Variables|/Game/UI/UI_PopUp_Mission.UI_PopUp_Mission_C|SetProgress _asui_pop_up_mission (Math|Float|Clamp(Float) (/ (Variables|Default|GetMaxDistance) (Math|Vector|Distance(Vector) (Transformation|GetWorldLocation (Variables|/Script/Engine.Actor|GetRootComponent _player)) (Transformation|GetWorldLocation (Variables|/Script/Engine.Actor|GetRootComponent (Variables|Default|GetDestination)))))))
        (if (>= (Math|Float|Clamp(Float) (/ (Variables|Default|GetMaxDistance) (Math|Vector|Distance(Vector) (Transformation|GetWorldLocation (Variables|/Script/Engine.Actor|GetRootComponent _player)) (Transformation|GetWorldLocation (Variables|/Script/Engine.Actor|GetRootComponent (Variables|Default|GetDestination)))))) 1.0)
          (CallFunction|EndMission)))
      (:else))))

(fn ConstructionScript
  (|CallParentFunction))