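; Mission progress display that tracks completed tasks across several objectives handlers and shows the count in a pop-up message widget.
; One second after BeginPlay it sums each handler's mission count into the total and registers itself with that handler.
; MissionValidated increments the completed count, refreshes the widget's title and text, and calls EndGame once the total is reached.
; EndGame currently only prints a debug string.
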(event EventBeginPlay
  (Utilities|FlowControl|Delay 1.0)
  (for _array_element (Variables|Default|GetObjectivesHandlers)
    (bind _output_get (Variables|Default|SetTotalTasks (+ (stale _output_get) (Variables|/Game/Blueprints/Missions/NewMissions/BP_ObjectivesDisplay.BP_ObjectivesDisplay_C|GetMissionsCount _array_element))))
    (Variables|/Game/Blueprints/Missions/NewMissions/BP_ObjectivesDisplay.BP_ObjectivesDisplay_C|SetBP_ObjectivesDisplayHandler _array_element self)))

(fn ConstructionScript)

(fn UpdateDisplay
  (bind _asui_pop_up_message (Utilities|Casting|CastToUI_PopUp_Message (UserInterface|GetWidget (Variables|Default|GetWidget))))
  (Variables|/Game/UI/UI_PopUp_Message.UI_PopUp_Message_C|SetMessageTitle _asui_pop_up_message (Variables|Default|GetTitleText))
  (Variables|/Game/UI/UI_PopUp_Message.UI_PopUp_Message_C|SetMessageContent _asui_pop_up_message (Utilities|String|Append (Variables|Default|GetDisplayText) (Utilities|String|ToString(Integer) (Variables|Default|GetCurrentTasks)) " / " (Utilities|String|ToString(Integer) (Variables|Default|GetTotalTasks)) " tasks completed")))

(fn MissionValidated
  (bind _result (Math|Integer|IncrementInt (Variables|Default|GetCurrentTasks))
    (:%20%20
      (CallFunction|UpdateDisplay)
      (if (>= _result (Variables|Default|GetTotalTasks))
        (CallFunction|EndGame)))))

(fn EndGame
  (Development|PrintString "end game"))