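; BP_MissionZone is a box trigger for a mission, showing its popup actor while the player overlaps it, until the mission is done.
; Once a player is cached from an overlap, Tick eases the popup toward them beyond a set distance, keeping it above their height.
; EndMission flags completion, updates the popup widget's text and progress with a delay value, and notifies the ObjectivesHandler.
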(event OnComponentBeginOverlap(Box)
  (params (OverlappedComponent :type Primitive%20Component%20Object%20Reference) (OtherActor :type Actor%20Object%20Reference) (OtherComp :type Primitive%20Component%20Object%20Reference) (OtherBodyIndex :type Integer) (bFromSweep :type Boolean) (SweepResult :type Hit%20Result%20Structure%20%28by%20ref%29))
  (if (not (Variables|Default|GetMissionDone))
    (bind _asbp_player (Utilities|Casting|CastToBP_Player OtherActor))
    (CallFunction|ShowMission false)
    (Variables|Default|SetPlayer _asbp_player)))

(event OnComponentEndOverlap(Box)
  (params (OverlappedComponent :type Primitive%20Component%20Object%20Reference) (OtherActor :type Actor%20Object%20Reference) (OtherComp :type Primitive%20Component%20Object%20Reference) (OtherBodyIndex :type Integer))
  (bind _asbp_player (Utilities|Casting|CastToBP_Player OtherActor))
  (CallFunction|ShowMission true)
  (Variables|Default|SetPlayer _asbp_player))

(event EventTick
  (params (DeltaSeconds :type Float%20%28single-precision%29))
  (bind _missionpopup (Variables|Default|GetMissionPopup))
  (bind _rootcomponent (Variables|/Script/Engine.Actor|GetRootComponent _missionpopup))
  (bind _returnvalue (Transformation|GetWorldLocation _rootcomponent))
  (bind _player (Variables|Default|GetPlayer)
    (:then
      (if (>= (Math|Vector|VectorLength (- (Transformation|GetWorldLocation (Variables|/Script/Engine.Actor|GetRootComponent _player)) _returnvalue)) (Variables|Default|GetPopUpDistance))
        (Transformation|SetWorldLocation _rootcomponent (Math|Vector|MakeVector (.x (+ _returnvalue (* (Math|Vector|Normalize (- (Transformation|GetWorldLocation (Variables|/Script/Engine.Actor|GetRootComponent _player)) _returnvalue)) (/ (Math|Vector|VectorLength (- (Transformation|GetWorldLocation (Variables|/Script/Engine.Actor|GetRootComponent _player)) _returnvalue)) 1e+02)))) (.y (+ _returnvalue (* (Math|Vector|Normalize (- (Transformation|GetWorldLocation (Variables|/Script/Engine.Actor|GetRootComponent _player)) _returnvalue)) (/ (Math|Vector|VectorLength (- (Transformation|GetWorldLocation (Variables|/Script/Engine.Actor|GetRootComponent _player)) _returnvalue)) 1e+02)))) (+ (.z (Transformation|GetWorldLocation (Variables|/Script/Engine.Actor|GetRootComponent _player))) 6.5e+02)) false false)))
    (:else)))

(fn ConstructionScript)

(fn ShowMission
  (params (Hidden :type Boolean))
  (Rendering|SetActorHiddenInGame (Variables|Default|GetMissionPopup) Hidden))

(fn EndMission
  (Variables|Default|SetMissionDone true)
  (bind _asbp_mission_pop_up (Utilities|Casting|CastToBP_MissionPopUp (Variables|Default|GetMissionPopup)))
  (bind _asui_pop_up_mission (Utilities|Casting|CastToUI_PopUp_Mission (UserInterface|GetUserWidgetObject (Variables|/Game/Blueprints/Missions/NewMissions/BP_MissionPopUp.BP_MissionPopUp_C|GetMissionWidget _asbp_mission_pop_up))))
  (Default|CompleteMission _asui_pop_up_mission (Variables|Default|GetDestroyPopUpDelay))
  (Variables|/Game/UI/UI_PopUp_Mission.UI_PopUp_Mission_C|SetMissionProgressText _asui_pop_up_mission (Variables|Default|GetMissionTextComplete))
  (Variables|/Game/UI/UI_PopUp_Mission.UI_PopUp_Mission_C|SetProgress _asui_pop_up_mission 1.0)
  (Default|MissionValidated (Variables|Default|GetObjectivesHandler) self))