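; Objectives display that tracks completed mission zones and shows a "tasks completed" counter on a UI_PopUp_Message widget.
; On BeginPlay it registers itself as each assigned mission's handler, stores the total, then empties the Missions array to reuse it as the completed list.
; Each first-time validation adds the zone, refreshes the title and count, and notifies BPObjectivesDisplayHandler.
; FirstCommunicationWithMaster returns the mission total.
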(event EventBeginPlay
  (bind _missions (Variables|Default|GetMissions))
  (Utilities|FlowControl|Sequence
    (:then_0
      (for _array_element _missions
        (Variables|/Game/Blueprints/Missions/NewMissions/BP_MissionZone.BP_MissionZone_C|SetObjectivesHandler _array_element self))
      (Variables|Default|SetMissionsCount (Utilities|Array|Length _missions))
      (Utilities|Array|Clear _missions))
    (:then_1
      (CallFunction|UpdateDisplay))))

(fn ConstructionScript)

(fn MissionValidated
  (params (Mission%20zone%20origin :type BP%20Mission%20Zone%20Object%20Reference))
  (bind _missions (Variables|Default|GetMissions))
  (if (not (Utilities|Array|ContainsItem _missions Mission%20zone%20origin))
    (Utilities|Array|Add _missions 0)
    (CallFunction|UpdateDisplay)
    (Default|MissionValidated (Variables|Default|GetBP_ObjectivesDisplayHandler))))

(fn UpdateDisplay
  (bind _asui_pop_up_message (Utilities|Casting|CastToUI_PopUp_Message (UserInterface|GetWidget (Variables|Default|GetWidget))))
  (Variables|/Game/UI/UI_PopUp_Message.UI_PopUp_Message_C|SetMessageTitle _asui_pop_up_message (Variables|Default|GetTitleText))
  (Variables|/Game/UI/UI_PopUp_Message.UI_PopUp_Message_C|SetMessageContent _asui_pop_up_message (Utilities|String|Append (Variables|Default|GetDisplayText) (Utilities|String|ToString(Integer) (Utilities|Array|Length (Variables|Default|GetMissions))) " / " (Utilities|String|ToString(Integer) (Variables|Default|GetMissionsCount)) " tasks completed")))

(fn FirstCommunicationwithMaster
  (return (Variables|Default|GetMissionsCount)))