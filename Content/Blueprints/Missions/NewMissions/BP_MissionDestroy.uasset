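; BP_MissionDestroy is a mission Blueprint that completes once every object in its ObjectsToDestroy list is destroyed.
; A looping one-second timer counts the list entries that are no longer valid while the mission is not done.
; It pushes the title, text and destroyed ratio to the UI_PopUp_Mission widget through BP_MissionPopUp.
; It calls EndMission when the count matches the list length, otherwise resets the counter for the next check.
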(event Custom|CheckArray
  (bind _objectstodestroy (Variables|Default|GetObjectsToDestroy))
  (if (not (Variables|Default|GetMissionDone))
    (for _array_element _objectstodestroy
      (Utilities|IsValid _array_element
        (:Is%20Not%20Valid
          (Math|Integer|IncrementInt (Variables|Default|GetCounter)))))
    (Utilities|FlowControl|Sequence
      (:then_0
        (bind _asbp_mission_pop_up (Utilities|Casting|CastToBP_MissionPopUp (Variables|Default|GetMissionPopup)))
        (bind _asui_pop_up_mission (Utilities|Casting|CastToUI_PopUp_Mission (UserInterface|GetUserWidgetObject (Variables|/Game/Blueprints/Missions/NewMissions/BP_MissionPopUp.BP_MissionPopUp_C|GetMissionWidget _asbp_mission_pop_up))))
        (Variables|/Game/UI/UI_PopUp_Mission.UI_PopUp_Mission_C|SetMissionTitle _asui_pop_up_mission (Variables|Default|GetMissionTitle))
        (Variables|/Game/UI/UI_PopUp_Mission.UI_PopUp_Mission_C|SetMissionProgressText _asui_pop_up_mission (Variables|Default|GetMissionText))
        (Variables|/Game/UI/UI_PopUp_Mission.UI_PopUp_Mission_C|SetProgress _asui_pop_up_mission (/ (Variables|Default|GetCounter) (Utilities|Array|Length (Variables|Default|GetObjectsToDestroy)))))
      (:then_1
        (if (== (Variables|Default|GetCounter) (Utilities|Array|Length _objectstodestroy))
          (CallFunction|EndMission)
          (else
            (Variables|Default|SetCounter 0)))))))

(event EventBeginPlay
  (Utilities|Time|SetTimerbyEvent (delegate Custom|CheckArray) 1.0 true))

(fn ConstructionScript
  (|CallParentFunction))