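; Mission Blueprint for opening a file, tracking a target file's approach to an action zone and showing progress in a popup.
; Each tick until done, it pushes title, text and progress to the popup's widget.
; Progress sums two clamped inverse-distance terms, player-to-file and file-to-zone, capped at 90% combined.
; When the target file is no longer valid, it calls EndMission.
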(event EventTick
  (params (DeltaSeconds :type Float%20%28single-precision%29))
  (bind _targetfile (Variables|Default|GetTargetFile))
  (bind _maxdistance (Variables|Default|GetMaxDistance))
  (bind _rootcomponent (Variables|/Script/Engine.Actor|GetRootComponent _targetfile))
  (bind _returnvalue (Transformation|GetWorldLocation _rootcomponent))
  (if (not (Variables|Default|GetMissionDone))
    (Variables|Default|GetPlayer
      (:then
        (bind _asbp_mission_pop_up (Utilities|Casting|CastToBP_MissionPopUp (Variables|Default|GetMissionPopup)))
        (bind _asui_pop_up_mission (Utilities|Casting|CastToUI_PopUp_Mission (UserInterface|GetUserWidgetObject (Variables|/Game/Blueprints/Missions/NewMissions/BP_MissionPopUp.BP_MissionPopUp_C|GetMissionWidget _asbp_mission_pop_up))))
        (Variables|/Game/UI/UI_PopUp_Mission.UI_PopUp_Mission_C|SetMissionTitle _asui_pop_up_mission (Variables|Default|GetMissionTitle))
        (Variables|/Game/UI/UI_PopUp_Mission.UI_PopUp_Mission_C|SetMissionProgressText _asui_pop_up_mission (Variables|Default|GetMissionText))
        (Variables|Default|GetTargetFile
          (:then
            (Variables|/Game/UI/UI_PopUp_Mission.UI_PopUp_Mission_C|SetProgress _asui_pop_up_mission (+ (Math|Float|Clamp(Float) (/ _maxdistance (Math|Vector|Distance(Vector) (Transformation|GetWorldLocation (Variables|/Script/Engine.Actor|GetRootComponent (Variables|Default|GetPlayer))) _returnvalue)) 0.0 0.45) (Math|Float|Clamp(Float) (/ _maxdistance (Math|Vector|Distance(Vector) _returnvalue (Transformation|GetWorldLocation (Variables|/Script/Engine.Actor|GetRootComponent (Variables|Default|GetTargetActionZone))))) 0.0 0.45))))
          (:else
            (CallFunction|EndMission))))
      (:else))))

(fn ConstructionScript
  (|CallParentFunction))