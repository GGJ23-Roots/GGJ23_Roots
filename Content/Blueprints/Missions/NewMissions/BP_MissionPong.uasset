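; BP_MissionPong is a mission Blueprint tied to a Pong object, displaying its title, text and progress in a mission pop-up.
; On BeginPlay it registers itself with the referenced Pong.
; Until MissionDone is set, Tick writes the title and text into the pop-up's UI_PopUp_Mission widget every frame.
; SetProgress writes a supplied progress value to the same widget.
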(event EventTick
  (params (DeltaSeconds :type Float%20%28single-precision%29))
  (if (not (Variables|Default|GetMissionDone))
    (bind _asbp_mission_pop_up (Utilities|Casting|CastToBP_MissionPopUp (Variables|Default|GetMissionPopup)))
    (bind _asui_pop_up_mission (Utilities|Casting|CastToUI_PopUp_Mission (UserInterface|GetUserWidgetObject (Variables|/Game/Blueprints/Missions/NewMissions/BP_MissionPopUp.BP_MissionPopUp_C|GetMissionWidget _asbp_mission_pop_up))))
    (Variables|/Game/UI/UI_PopUp_Mission.UI_PopUp_Mission_C|SetMissionTitle _asui_pop_up_mission (Variables|Default|GetMissionTitle))
    (Variables|/Game/UI/UI_PopUp_Mission.UI_PopUp_Mission_C|SetMissionProgressText _asui_pop_up_mission (Variables|Default|GetMissionText))))

(event EventBeginPlay
  (bind _pong (Variables|Default|GetPong)
    (:then
      (Variables|/Game/Blueprints/Pong/BP_Pong.BP_Pong_C|SetMissionPong _pong self))
    (:else)))

(fn ConstructionScript
  (|CallParentFunction))

(fn SetProgress
  (params (Progress :type Float%20%28double-precision%29))
  (bind _asbp_mission_pop_up (Utilities|Casting|CastToBP_MissionPopUp (Variables|Default|GetMissionPopup)))
  (bind _asui_pop_up_mission (Utilities|Casting|CastToUI_PopUp_Mission (UserInterface|GetUserWidgetObject (Variables|/Game/Blueprints/Missions/NewMissions/BP_MissionPopUp.BP_MissionPopUp_C|GetMissionWidget _asbp_mission_pop_up))))
  (Variables|/Game/UI/UI_PopUp_Mission.UI_PopUp_Mission_C|SetProgress _asui_pop_up_mission Progress))