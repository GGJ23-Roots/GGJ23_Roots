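; Mission handler actor that runs a sequence of mission objects and prints each one's text.
; BeginPlay shows the first text and starts the first object through BPI_MissionObject, passing itself as handler.
; ValidateMission increments CurrentMission and prints the matching text, but always calls StartMission on element zero rather than the current index.
; An empty or exhausted list calls EndGame, which only prints a message.
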(event EventBeginPlay
  (if (!= (Utilities|Array|Length (Variables|Default|GetMissionObjects)) 0)
    (CallFunction|DisplayMissionText)
    (bind _asbpi_mission_object (Utilities|Casting|CastToBPI_MissionObject (Utilities|Array|Get(acopy) (Variables|Default|GetMissionObjects))))
    (Default|StartMission _asbpi_mission_object self)
    (else
      (CallFunction|EndGame))))

(fn ConstructionScript)

(fn ValidateMission
  (bind _result (Math|Integer|IncrementInt (Variables|Default|GetCurrentMission))
    (:%20%20
      (if (< _result (Utilities|Array|Length (Variables|Default|GetMissionObjects)))
        (CallFunction|DisplayMissionText _result)
        (bind _asbpi_mission_object (Utilities|Casting|CastToBPI_MissionObject (Utilities|Array|Get(acopy) (Variables|Default|GetMissionObjects))))
        (Default|StartMission _asbpi_mission_object self)
        (else
          (CallFunction|EndGame))))))

(fn DisplayMissionText
  (params (MissionIndex :type Integer))
  (Development|PrintString (Utilities|Array|Get(acopy) (Variables|Default|GetMissionTexts) MissionIndex)))

(fn EndGame
  (Development|PrintString "End game"))