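; Legacy music mixer Blueprint that drives phase changes across its set of music players on fixed timers.
; BeginPlay starts two one-shot timers, each firing a custom event that loops over MusicPlayers and calls PlayMusicPhase with a different phase enum value.
; Debug prints label the first switch as the main phase and the later one as the outro, so the timing appears hard-coded for testing.
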(event Custom|CustomEvent
  (bind _result (Utilities|Set|ToArray (Variables|Default|GetMusicPlayers)))
  (for _array_element _result
    (Default|PlayMusicPhase _array_element "NewEnumerator1")
    (Development|PrintString "WILL PLAY MAIN")))

(event Custom|CustomEvent_0
  (bind _result (Utilities|Set|ToArray (Variables|Default|GetMusicPlayers)))
  (for _array_element _result
    (Default|PlayMusicPhase _array_element "NewEnumerator2")
    (Development|PrintString "WILL PLAY OUTRO")))

(event EventBeginPlay
  (Development|PrintString "OK")
  (Utilities|Time|SetTimerbyEvent (delegate Custom|CustomEvent) 3.0)
  (Utilities|Time|SetTimerbyEvent (delegate Custom|CustomEvent_0) 6.0))

(fn ConstructionScript)