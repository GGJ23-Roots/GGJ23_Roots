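; Legacy music player with intro, main and outro audio components, optionally started on BeginPlay.
; Play starts every idle component together, while SetVolumeMultiplier mutes all but the current phase's track.
; The intro's finished event, bound after a short timer delay, switches to main.
; Tick ramps volume by VolumeLerpSpeed without reading TargetVolumeMultiplier, so Stop setting it to zero never fades out; debug prints remain.
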(event Custom|OnIntroFinished
  (CallFunction|Play "NewEnumerator1")
  (Development|PrintString "OKAY" true true "(R=1.000000,G=0.790901,B=0.000000,A=1.000000)"))

(event Custom|CustomEvent
  (EventDispatchers|BindEventtoOnAudioFinished (Variables|Components|GetAudioComp_Intro) (delegate Custom|OnIntroFinished)))

(event EventBeginPlay
  (Utilities|Time|SetTimerbyEvent (delegate Custom|CustomEvent) 0.5)
  (Utilities|FlowControl|Sequence
    (:then_0
      (Audio|Components|Audio|SetSound (Variables|Components|GetAudioComp_Intro) (Variables|Default|GetSound_Intro))
      (Audio|Components|Audio|SetSound (Variables|Components|GetAudioComp_Main) (Variables|Default|GetSound_Main))
      (Audio|Components|Audio|SetSound (Variables|Components|GetAudioComp_Outro) (Variables|Default|GetSound_Outro))
      (CallFunction|SetVolumeMultiplier 0.0))
    (:then_1
      (if (Variables|Default|GetPlayOnStartup)
        (CallFunction|Play "NewEnumerator0")
        (else
          (CallFunction|Stop))))))

(event EventTick
  (params (DeltaSeconds :type Float%20%28single-precision%29))
  (bind _output_get (Variables|Default|Set_CurrentVolumeMultiplier (Math|Float|Clamp(Float) (+ (* DeltaSeconds (Variables|Default|GetVolumeLerpSpeed)) (Variables|Default|Get_CurrentVolumeMultiplier)))))
  (CallFunction|SetVolumeMultiplier _output_get)
  (Development|PrintString (Utilities|String|ToString(Float) _output_get) true true "(R=1.000000,G=0.000000,B=0.037674,A=1.000000)" 0.1)
  (Development|PrintString (Utilities|String|EnumtoString (Variables|Default|Get_CurrentMusicPhase)) true true "(R=0.000000,G=0.660000,B=1.000000,A=1.000000)" 0.1))

(fn ConstructionScript)

(fn Play
  (params (Phase :type EMusicPhase%20Enum :default "NewEnumerator3"))
  (bind _audiocomp_intro (Variables|Components|GetAudioComp_Intro))
  (bind _audiocomp_main (Variables|Components|GetAudioComp_Main))
  (bind _audiocomp_outro (Variables|Components|GetAudioComp_Outro))
  (Variables|Default|Set_CurrentMusicPhase Phase)
  (Utilities|FlowControl|Sequence
    (:then_0
      (if (not (Audio|Components|Audio|IsPlaying _audiocomp_intro))
        (Audio|Components|Audio|Play _audiocomp_intro 0.0)
        (LocalVariables|SetNowPlaying true :!label _label)))
    (:then_1
      (if (not (Audio|Components|Audio|IsPlaying _audiocomp_main))
        (Audio|Components|Audio|Play _audiocomp_main 0.0)
        (goto _label)))
    (:then_2
      (if (not (Audio|Components|Audio|IsPlaying _audiocomp_outro))
        (Audio|Components|Audio|Play _audiocomp_outro 0.0)
        (goto _label)))
    (:then_3
      (Variables|Default|Set_TargetVolumeMultiplier 1.0)
      (return (LocalVariables|GetNowPlaying)))))

(fn Stop
  (Variables|Default|Set_TargetVolumeMultiplier 0.0)
  (bind _output_get (LocalVariables|SetNowStopped (CallFunction|IsPlaying)))
  (return _output_get))

(fn IsPlaying
  (bind _audiocomp_intro (Variables|Components|GetAudioComp_Intro))
  (bind _audiocomp_main (Variables|Components|GetAudioComp_Main))
  (bind _audiocomp_outro (Variables|Components|GetAudioComp_Outro))
  (return (Math|Boolean|ORBoolean (and (Audio|Components|Audio|IsPlaying _audiocomp_intro) (> (Variables|/Script/Engine.AudioComponent|GetVolumeMultiplier _audiocomp_intro) 0.0)) (and (Audio|Components|Audio|IsPlaying _audiocomp_main) (> (Variables|/Script/Engine.AudioComponent|GetVolumeMultiplier _audiocomp_main) 0.0)) (and (Audio|Components|Audio|IsPlaying _audiocomp_outro) (> (Variables|/Script/Engine.AudioComponent|GetVolumeMultiplier _audiocomp_outro) 0.0)))))

(fn SetVolumeMultiplier
  (params (Multiplier :type Float%20%28double-precision%29))
  (Utilities|FlowControl|Sequence
    (:then_0
      (Variables|/Script/Engine.AudioComponent|SetVolumeMultiplier (Variables|Components|GetAudioComp_Intro) (Math|Float|SelectFloat Multiplier 0.0 (Utilities|Enum|Equal(Enum) (Variables|Default|Get_CurrentMusicPhase) "NewEnumerator0"))))
    (:then_1
      (Variables|/Script/Engine.AudioComponent|SetVolumeMultiplier (Variables|Components|GetAudioComp_Main) (Math|Float|SelectFloat Multiplier 0.0 (Utilities|Enum|Equal(Enum) (Variables|Default|Get_CurrentMusicPhase) "NewEnumerator1"))))
    (:then_2
      (Variables|/Script/Engine.AudioComponent|SetVolumeMultiplier (Variables|Components|GetAudioComp_Outro) (Math|Float|SelectFloat Multiplier 0.0 (Utilities|Enum|Equal(Enum) (Variables|Default|Get_CurrentMusicPhase) "NewEnumerator2"))))))