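; BP_MusicMixer is a music player that layers tracks on separate audio components and crossfades between them, optionally starting one on BeginPlay.
; Play searches for an existing player, otherwise adds and starts a new component, muting all but the first.
; RaiseVolume, not called within this graph, steps the chosen component's volume up and all others down by VolumeLerpSpeed times delta time, without clamping.
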(event EventBeginPlay
  (bind _sound_to_play_on_startup (Variables|Default|GetSound%20To%20Play%20On%20Startup))
  (if (Utilities|IsValid _sound_to_play_on_startup)
    (CallFunction|Play _sound_to_play_on_startup)))

(fn ConstructionScript)

(fn Play
  (params (Music :type Sound%20Cue%20Object%20Reference))
  (bind _array_element (Utilities|Array|ForEachLoopwithBreak (Variables|Default|GetAudioComponents) :!label _label)
    (:LoopBody
      (if (== _array_element Music)
        (LocalVariables|SetFoundMusicPlayer true)
        (goto _label Break)))
    (:Completed
      (if (not (LocalVariables|GetFoundMusicPlayer))
        (bind _returnvalue (AddComponent|AddAudioComponent true (Transformation|GetActorTransform)))
        (bind _returnvalue_2 (Utilities|Array|Add (Variables|Default|GetAudioComponents) _returnvalue))
        (Audio|Components|Audio|SetSound _returnvalue Music)
        (Audio|Components|Audio|Play _returnvalue 0.0)
        (Variables|Default|Set_PlayingAudioComponentIndex _returnvalue_2)
        (if (not (== _returnvalue_2 0))
          (Audio|Components|Audio|SetVolumeMultiplier _returnvalue 0.0 :!class /Script/Engine.AudioComponent))))))

(fn RaiseVolume
  (params (Audio%20Component :type Audio%20Component%20Object%20Reference) (Delta%20Time :type Float%20%28double-precision%29))
  (bind _volumelerpspeed (Variables|Default|GetVolumeLerpSpeed))
  (bind _returnvalue (* _volumelerpspeed Delta%20Time))
  (for (_array_element _array_index) (Variables|Default|GetAudioComponents)
    (if (== _array_element Audio%20Component)
      (Variables|Default|Set_PlayingAudioComponentIndex _array_index)
      (Audio|Components|Audio|SetVolumeMultiplier _array_element (+ (Variables|/Script/Engine.AudioComponent|GetVolumeMultiplier _array_element) _returnvalue) :!class /Script/Engine.AudioComponent)
      (else
        (Audio|Components|Audio|SetVolumeMultiplier _array_element (- (Variables|/Script/Engine.AudioComponent|GetVolumeMultiplier _array_element) _returnvalue) :!class /Script/Engine.AudioComponent)))))