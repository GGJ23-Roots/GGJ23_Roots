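; BP_MusicPlayer plays music in phases (Intro, Main, Outro, None), cycling through a sound list for each, and can start with Intro on BeginPlay.
; The audio component's playback-percent event triggers the next part shortly before the current one ends.
; PlayMusicPhase queues a target phase, so switches wait for that point unless nothing is playing.
; The first Intro uses pre-intro sounds; reaching None stops playback and resets that.
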(event Custom|OnAudioPlaybackPercentChange
  (params (PlayingSoundWave :type Sound%20Wave%20Object%20Reference) (PlaybackPercent :type Float%20%28single-precision%29))
  (Development|PrintString (Utilities|String|ToString(Float) PlaybackPercent))
  (if (<= (- 1.0 PlaybackPercent) (Variables|Default|GetPlaybackPercentOffset))
    (CallFunction|PlayNextPart)))

(event EventBeginPlay
  (EventDispatchers|BindEventtoOnAudioPlaybackPercent (Variables|Default|GetAudioComponent) (delegate Custom|OnAudioPlaybackPercentChange))
  (if (Variables|Default|GetPlayOnStartup)
    (CallFunction|PlayMusicPhase "NewEnumerator0")))

(fn ConstructionScript)

(fn PlayMusicPhase
  (params (Phase :type EMusicPhase%20Enum :default "NewEnumerator0"))
  (Variables|Default|Set_TargetMusicPhase Phase)
  (if (not (Audio|Components|Audio|IsPlaying (Variables|Default|GetAudioComponent)))
    (CallFunction|PlayNextPart)))

(fn Stop
  (Audio|Components|Audio|Stop (Variables|Default|GetAudioComponent))
  (Variables|Default|Set_SoundIndex 0))

(fn PlayNextPart
  (if (Utilities|Enum|Equal(Enum) (Variables|Default|Get_CurrentMusicPhase) (Variables|Default|Get_TargetMusicPhase))
    (if (Utilities|Enum|NotEqual(Enum) (Variables|Default|Get_TargetMusicPhase) "NewEnumerator3")
      (bind _result (Math|Integer|IncrementInt (Variables|Default|Get_SoundIndex) :!label _label)
        (:%20%20
          (bind _output_get (Variables|Default|Set_SoundIndex _result))
          (if (< _output_get (Utilities|Array|Length (Variables|Default|Get_CurrentSounds)))
            _
            (else
              (bind _output_get_2 (Variables|Default|Set_SoundIndex 0))))
          (Audio|Components|Audio|SetSound (Variables|Default|GetAudioComponent) (Utilities|Array|Get(acopy) (Variables|Default|Get_CurrentSounds) _output_get_2))
          (Audio|Components|Audio|Play (Variables|Default|GetAudioComponent) 0.0)))
      (else
        (bind _output_get_3 (Variables|Default|Set_CurrentMusicPhase (Variables|Default|Get_TargetMusicPhase) :!label _label_2))
        (switch Utilities|FlowControl|Switch|SwitchonEMusicPhase _output_get_3
          (:NewEnumerator3
            (CallFunction|Stop)
            (Variables|Default|Set_DidPlayPreIntro false)
            (Development|PrintString "STOPPING MUSIC PLAYER"))
          (:NewEnumerator0
            (if (Variables|Default|Get_DidPlayPreIntro)
              (Variables|Default|Set_CurrentSounds (Variables|Default|GetSounds_Intro))
              (else
                (Variables|Default|Set_DidPlayPreIntro true)
                (Variables|Default|Set_CurrentSounds (Variables|Default|GetSounds_PreIntro))))
            (Variables|Default|Set_SoundIndex -1 :!label _label_3)
            (goto _label))
          (:NewEnumerator1
            (Variables|Default|Set_CurrentSounds (Variables|Default|GetSounds_Main))
            (goto _label_3))
          (:NewEnumerator2
            (Variables|Default|Set_CurrentSounds (Variables|Default|GetSounds_Outro))
            (goto _label_3)))))
    (else
      (goto _label_2))))